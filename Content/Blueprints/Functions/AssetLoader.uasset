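; Function library that loads data-driven RTS object definitions from .cfg files into server and client object structs.
; Server loading scans each configured directory, parses key=value lines into properties, derives requirements, and takes the ID from the filename and type from the directory's matching enum.
; Client loading extends a server object by resolving its model and shader properties to mesh and material assets, and reading its texture from a PNG at runtime.
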(fn `LoadClientObject`
  (params (Array :type "/Game/Structs/ServerObject Structure (by ref)"))
  (returns (Object :type "/Game/Structs/ClientObject Structure"))
  (bind (_id _requirements _properties _type) (break `/Game/Structs/ServerObject` Array))
  (return (make `/Game/Structs/ClientObject` _id (`RtsFunctions.FindStaticMesh` (`KismetStringLibrary.Concat_StrStr` "/Game/Models/" (`RtsFunctions.GetValueOfProperty` _properties "model"))) (`RtsFunctions.ReadPNGFile` (`KismetStringLibrary.Concat_StrStr` "Content/RTS/Textures/" (`RtsFunctions.GetValueOfProperty` _properties "texture") ".png")) (`RtsFunctions.FindMaterial` (`KismetStringLibrary.Concat_StrStr` "/Game/Materials/" (`RtsFunctions.GetValueOfProperty` _properties "shader"))) _requirements _properties _type)))

(fn `LoadPropertiesAndRequirements`
  (params (File :type String))
  (returns (Requirements :type "Array of /Game/Structs/Requirement Structure") (Properties :type "Array of StringPair Structure"))
  (locals (ValueList :type "Array of StringPair Structure"))
  (bind _valuelist (`local.ValueList`))
  (for _array_element (`RtsFunctions.SeperateLines` (`RtsFunctions.ReadStringFromFile` File))
    (bind (_lefts _rights) (`KismetStringLibrary.Split` _array_element "="))
    (`KismetArrayLibrary.Array_Add` (`local.ValueList`) (make `StringPair` _lefts _rights)))
  (return (`/Game/Blueprints/Functions/CountArrayFunctions.Get Requirements from Properties` _valuelist) _valuelist))

(fn `LoadServerObjects`
  (returns (Objects :type "Array of /Game/Structs/ServerObject Structure"))
  (locals (Paths :type "Array of String") (PathEnums :type "Array of /Game/Structs/ContentType Enum") (List :type "Array of /Game/Structs/ServerObject Structure"))
  (for (_array_element _array_index) (`local.Paths`)
    (for _array_element_2 (`RtsFunctions.FindAllFilesInDirectory` _array_element ".cfg")
      (bind (_requirements _properties) (`self.LoadPropertiesAndRequirements` (`KismetStringLibrary.Concat_StrStr` _array_element _array_element_2)))
      (`KismetArrayLibrary.Array_Add` (`local.List`) (make `/Game/Structs/ServerObject` (`KismetStringLibrary.Split` _array_element_2 "." "IgnoreCase" "FromEnd") _requirements _properties (`KismetArrayLibrary.Array_Get` (`local.PathEnums`) _array_index)))))
  (return (`local.List`)))