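; Blueprint function library of quadratic Bezier curve helpers for 2D and 3D points.
; BezierQuad2D and BezierQuad3D evaluate the curve at T from three control points, using two nested linear interpolations written as weighted sums.
; A separate helper, Func, returns the difference vectors from Start to Mid and from Mid to End.
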(fn `BezierQuad2D`
  (params (t :type "Float (double-precision)") (p1 :type "Vector2D Structure") (p2 :type "Vector2D Structure") (p3 :type "Vector2D Structure"))
  (returns (b :type "Vector2D Structure"))
  (bind _returnvalue (- 1.0 t))
  (return (+ (* (+ (* p1 _returnvalue) (* p2 t)) _returnvalue) (* (+ (* p2 _returnvalue) (* p3 t)) t))))

(fn `BezierQuad3D`
  (params (t :type "Float (double-precision)") (P1 :type "Vector Structure") (P2 :type "Vector Structure") (P3 :type "Vector Structure"))
  (returns (b :type "Vector Structure"))
  (bind _returnvalue (- 1.0 t))
  (return (+ (* (+ (* P1 _returnvalue) (* P2 t)) _returnvalue) (* (+ (* P2 _returnvalue) (* P3 t)) t))))

(fn `func`
  (params (Start :type "Vector Structure") (Mid :type "Vector Structure") (End :type "Vector Structure"))
  (returns (t1 :type "Vector Structure") (t2 :type "Vector Structure"))
  (return (- Mid Start) (- End Mid)))