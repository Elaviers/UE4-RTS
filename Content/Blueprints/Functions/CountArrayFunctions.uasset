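; Function library for counting buildings by type in BuildingCounter arrays, tracking total and constructed amounts, and for building requirement lists.
; The add functions update the matching entry and return its previous value, or append a new one; a new constructed entry also counts toward the total.
; Lookups return zero or -1 total for missing names, depending on Safe.
; Requirements come from splitting property names at the last dash into ID and "count" or "min" type.
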(fn `Add To Constructed`
  (params (Array :type "Array of /Game/Structs/BuildingCounter Structure (by ref)") (Name :type String) (Value :type Integer))
  (returns (`New Value` :type Integer))
  (for (_array_element _array_index) Array
    (bind (_type _total _constructed) (break `/Game/Structs/BuildingCounter` _array_element))
    (if (`KismetStringLibrary.EqualEqual_StrStr` _type Name)
      (`KismetArrayLibrary.Array_Set` Array _array_index (make `/Game/Structs/BuildingCounter` Name _total (+ _constructed Value)))
      (return _constructed)))
  (`KismetArrayLibrary.Array_Add` Array (make `/Game/Structs/BuildingCounter` Name Value Value))
  (return Value))

(fn `Add To Total`
  (params (Array :type "Array of /Game/Structs/BuildingCounter Structure (by ref)") (Name :type String) (Value :type Integer))
  (returns (`New Value` :type Integer))
  (for (_array_element _array_index) Array
    (bind (_type _total _constructed) (break `/Game/Structs/BuildingCounter` _array_element))
    (if (`KismetStringLibrary.EqualEqual_StrStr` _type Name)
      (`KismetArrayLibrary.Array_Set` Array _array_index (make `/Game/Structs/BuildingCounter` Name (+ _total Value) _constructed))
      (return _total)))
  (`KismetArrayLibrary.Array_Add` Array (make `/Game/Structs/BuildingCounter` Name Value))
  (return Value))

(fn `Get Count of Name`
  (params (Array :type "Array of /Game/Structs/BuildingCounter Structure (by ref)") (Name :type String) (Safe :type Boolean :default false))
  (returns (Total :type Integer) (Constructed :type Integer))
  (for _array_element Array
    (bind (_type _total _constructed) (break `/Game/Structs/BuildingCounter` _array_element))
    (if (`KismetStringLibrary.EqualEqual_StrStr` _type Name)
      (return _total _constructed)))
  (if Safe
    (return 0 0)
    (else
      (return -1 0))))

(fn `Get Requirements from Properties`
  (params (Properties :type "Array of StringPair Structure (by ref)"))
  (returns (Requirements :type "Array of /Game/Structs/Requirement Structure"))
  (locals (Type :type "/Game/Structs/RequirementType Enum" :default "(())") (Array :type "Array of /Game/Structs/Requirement Structure"))
  (for _array_element Properties
    (bind (_property _value) (break `StringPair` _array_element))
    (bind (_lefts _rights) (`KismetStringLibrary.Split` _property "-" "IgnoreCase" "FromEnd"))
    (if (`KismetStringLibrary.EqualEqual_StrStr` _rights "count")
      (set `local.Type` "NewEnumerator1")
      (`KismetArrayLibrary.Array_Add` (`local.Array`) (make `/Game/Structs/Requirement` _lefts (`KismetStringLibrary.Conv_StringToInt` _value) (`local.Type`)) :!label _label)
      (elif (`KismetStringLibrary.EqualEqual_StrStr` _rights "min")
        (set `local.Type` "NewEnumerator0")
        (goto _label))))
  (return (`local.Array`)))