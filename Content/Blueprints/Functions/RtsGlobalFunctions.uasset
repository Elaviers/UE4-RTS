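; Blueprint function library of global RTS helpers for string map lookup and empty object construction.
; FindString returns the value stored under a key in a string map, or a supplied default when the key is missing.
; GetEmptyClientObject and GetEmptyServerObject build client and server object values with no requirements and an empty properties map.
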(fn `FindString`
  (params (StringMap :type "Map of String to String") (Key :type String) (Default :type String))
  (returns (Value :type String))
  (bind (_value _returnvalue) (`BlueprintMapLibrary.Map_Find` StringMap Key))
  (if _returnvalue
    (return _value)
    (else
      (return Default))))

(fn `GetEmptyClientObject`
  (returns (Object :type "/Game/Structs/ClientObject Structure"))
  (locals (`Empty Map` :type "Map of String to String"))
  (return (make `/Game/Structs/ClientObject` "" null null null (`|MakeArray`) (`local.Empty Map`))))

(fn `GetEmptyServerObject`
  (returns (Object :type "/Game/Structs/ServerObject Structure"))
  (locals (`Empty Map` :type "Map of String to String"))
  (return (make `/Game/Structs/ServerObject` "" (`|MakeArray`) (`local.Empty Map`))))