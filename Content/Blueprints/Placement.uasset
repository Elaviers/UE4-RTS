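; Placement logic for an RTS that previews and places buildings and roads, with a client event to toggle it.
; SetObject swaps the preview actor by type, Update moves it, and Place commits it.
; Buildings interpolate toward a spot offset to either side of the first road spline in range, aligned to it.
; Roads use a start, mid, end state machine, requesting server creation and chaining segments with carried-over tangents.
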(event `Set Enabled (Client)`
  (params (Enabled :type Boolean))
  (`self.SetEnabled` Enabled))

(fn `Notify of Count Change`
  (params (Name :type String)))

(fn `Place`
  (params (Location :type "Vector Structure"))
  (returns (Success :type Boolean))
  (locals (Incremented :type Boolean))
  (bind _roads (`self.Roads`))
  (bind _asroad_preview (cast `/Game/Actors/Road_Preview` (`self.Preview`) :!pure true))
  (bind (_pos1 _tan1 _pos2 _tan2) (`/Game/Actors/Road_Preview.info` _asroad_preview))
  (if (`self.Enabled`)
    (switch `/Game/Structs/ContentType` (`.Type_14_EFED544C4F7343C7C2DC1F9D744123DA` (break `/Game/Structs/ClientObject` (`self.CurrentObject`)))
      (:`NewEnumerator2`
        (return false))
      (:`NewEnumerator0`
        (bind _success (`/Game/Actors/Building_Preview.SpawnBuilding` (cast `/Game/Actors/Building_Preview` (`self.Preview`) :!pure true)))
        (return _success))
      (:`NewEnumerator1`
        (switch `int` (`self.RoadMode`)
          (:`0`
            (`/Game/Actors/Road_Preview.Set Start Point` _asroad_preview Location)
            (set `self.RoadMode` 1)
            (`/Game/Player/RtsPlayerController.Create Road On Server` (cast `/Game/Player/RtsPlayerController` (`GameplayStatics.GetPlayerController` 0) :!pure true) (`.ID_25_7A4E81A5419F763F158F18B5B4976B21` (break `/Game/Structs/ClientObject` (`self.CurrentObject`)))))
          (:`1`
            (set `self.RoadMode` 2))
          (:`2`
            (set `self.RoadMode` 1)
            (`/Game/Actors/Road_Preview.SpawnRoad` _asroad_preview (`KismetArrayLibrary.Array_Get` _roads (`KismetArrayLibrary.Array_LastIndex` _roads)))
            (`/Game/Actors/Road_Preview.Set Start Point` _asroad_preview _pos2)
            (`/Game/Actors/Road_Preview.Set Start Tangent` _asroad_preview (* (`KismetMathLibrary.Normal` _tan2) 2000.0))))
        (return true)))
    (else
      (return false))))

(fn `RoadSnap`
  (params (Roads :type "Array of /Game/Actors/Road Object Reference") (Transform :type "Transform Structure") (`Max Distance` :type "Float (double-precision)") (`Distance from Road` :type "Float (double-precision)"))
  (returns (Snapped :type "Transform Structure"))
  (bind _location (.location Transform))
  (for _array_element Roads
    (bind _roadspline (`/Game/Actors/Road.RoadSpline` _array_element))
    (bind _returnvalue (`SplineComponent.FindLocationClosestToWorldLocation` _roadspline _location "Local"))
    (bind _returnvalue_2 (- _location _returnvalue))
    (if (<= (`KismetMathLibrary.VSize` _returnvalue_2) `Max Distance`)
      (bind _returnvalue_3 (`SplineComponent.FindRotationClosestToWorldLocation` _roadspline _location "Local"))
      (bind _returnvalue_4 (`KismetMathLibrary.GetRightVector` _returnvalue_3))
      (if (> (`KismetMathLibrary.Dot_VectorVector` _returnvalue_2 _returnvalue_4) 0.0)
        (bind _returnvalue_5 (* _returnvalue_4 `Distance from Road`))
        (return (`KismetMathLibrary.MakeTransform` (+ _returnvalue _returnvalue_5) _returnvalue_3))
        (else
          (return (`KismetMathLibrary.MakeTransform` (- _returnvalue _returnvalue_5) (`KismetMathLibrary.ComposeRotators` _returnvalue_3 (struct :`Yaw` 180.0))))))))
  (return Transform))

(fn `Set Object`
  (params (Object :type "/Game/Structs/ClientObject Structure"))
  (bind (_id _mesh _texture _material _requirements _properties _type) (break `/Game/Structs/ClientObject` Object))
  (bind _preview (`self.Preview`))
  (set `self.CurrentObject` Object)
  (switch `/Game/Structs/ContentType` _type
    (:`NewEnumerator2`
      (`self.RemoveActor` _preview))
    (:`NewEnumerator0`
      (bind _transform (`self.RemoveActor` _preview)
        (:`  `
          (bind _returnvalue (`|SpawnActorFromClass` "/Game/Actors/Building_Preview.Building_Preview_C" _transform "Undefined" "OverrideRootScale"))
          (`/Game/Actors/Building_Preview.Create` _returnvalue _id)
          (set `self.Preview` _returnvalue))))
    (:`NewEnumerator1`
      (`self.RemoveActor` _preview
        (:`  `
          (bind _returnvalue_2 (`|SpawnActorFromClass` "/Game/Actors/Road_Preview.Road_Preview_C" (`KismetMathLibrary.MakeTransform` (0.0 0.0 0.0)) "Undefined" "OverrideRootScale"))
          (set `self.Preview` _returnvalue_2)
          (set `self.RoadMode` 0))))))

(fn `SetEnabled`
  (params (Enabled :type Boolean))
  (bind _preview (`self.Preview`))
  (bind _output_get (set `self.Enabled` Enabled))
  (`/Engine/EditorBlueprintResources/StandardMacros.IsValid` (`self.Preview`)
    (:`Is Valid`
      (if _output_get
        (`Actor.SetActorHiddenInGame` _preview false)
        (else
          (`Actor.SetActorHiddenInGame` _preview true))))))

(fn `Update`
  (params (Transform :type "Transform Structure") (DeltaSeconds :type "Float (double-precision)"))
  (bind _location (.location Transform))
  (bind _asroad_preview (cast `/Game/Actors/Road_Preview` (`self.Preview`) :!pure true))
  (bind (_pos1 _tan1 _pos2 _tan2 _mid) (`/Game/Actors/Road_Preview.info` _asroad_preview))
  (switch `/Game/Structs/ContentType` (`.Type_14_EFED544C4F7343C7C2DC1F9D744123DA` (break `/Game/Structs/ClientObject` (`self.CurrentObject`)))
    (:`NewEnumerator0`
      (bind _snapped (`self.RoadSnap` (`self.Roads`) Transform 512.0 400.0))
      (`Actor.K2_SetActorTransform` (`self.Preview`) (`KismetMathLibrary.TInterpTo` (`Actor.GetTransform` (`self.Preview`)) _snapped DeltaSeconds 16.0) false false))
    (:`NewEnumerator1`
      (switch `int` (`self.RoadMode`)
        (:`0`
          (`KismetSystemLibrary.DrawDebugSphere` _location 50.0 12 (struct :`R` 1.0 :`G` 0.008376 :`A` 1.0) 0.1 10.0))
        (:`1`
          (`/Game/Actors/Road_Preview.Set Mid Point` _asroad_preview _location true)
          (if (`self.Enabled`) :!label _label
            (`KismetSystemLibrary.DrawDebugLine` _pos1 _mid (struct :`R` 1.0 :`G` 0.038484 :`A` 1.0) 0.1 10.0)
            (`KismetSystemLibrary.DrawDebugLine` _pos2 _mid (struct :`G` 1.0 :`B` 0.05721 :`A` 1.0) 0.1 10.0)))
        (:`2`
          (`/Game/Actors/Road_Preview.Set End Point` _asroad_preview _location)
          (goto _label))))))