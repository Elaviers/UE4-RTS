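; RtsState is an RTS state Blueprint that loads and holds the current level's configuration properties.
; On BeginPlay it fills LevelProperties, if still empty, from a .cfg file in Content/RTS/Levels.
; The file name comes from the RTS instance's LevelID, falling back to a string read from a "level" file when that ID is empty.
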(event `self.ReceiveBeginPlay`
  (`self.LoadLevelProperties`))

(fn `LoadLevelProperties`
  (bind _levelid (`/Game/Blueprints/RTSInstance.LevelID` (`/Game/Blueprints/RtsMacros.GetRtsInstance`)))
  (if (== (`KismetArrayLibrary.Array_Length` (`self.LevelProperties`)) 0)
    (if (`KismetStringLibrary.EqualEqual_StrStr` _levelid)
      (bind _values (`/Game/Blueprints/AssetLoader.LoadProperties` (`KismetStringLibrary.Concat_StrStr` "Content/RTS/Levels/" (`RtsFunctions.ReadStringFromFile` "level") ".cfg")))
      (set `self.LevelProperties` _values)
      (else
        (bind _values_2 (`/Game/Blueprints/AssetLoader.LoadProperties` (`KismetStringLibrary.Concat_StrStr` "Content/RTS/Levels/" _levelid ".cfg")))
        (set `self.LevelProperties` _values_2)))))

(fn `UserConstructionScript`)