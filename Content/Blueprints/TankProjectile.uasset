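; Tank projectile actor that Fire launches by setting its physics sphere's velocity from a direction and power.
; On a hit, the authority spawns an explosion emitter, deactivates the trail, hides the sphere, ignores further collisions and damages the hit actor.
; Tick turns the trail along the velocity, and once the trail component is invalid the authority destroys the actor, so destruction waits on the trail.
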(event `Fire`
  (params (Direction :type "Vector Structure") (Power :type "Float (double-precision)"))
  (`PrimitiveComponent.SetPhysicsLinearVelocity` (`self.Sphere`) (* Direction Power) false "None"))

(event `self.ReceiveHit`
  (params (MyComp :type "PrimitiveComponent Object Reference") (Other :type "Actor Object Reference") (OtherComp :type "PrimitiveComponent Object Reference") (bSelfMoved :type Boolean) (HitLocation :type "Vector Structure") (HitNormal :type "Vector Structure") (NormalImpulse :type "Vector Structure") (Hit :type "HitResult Structure (by ref)"))
  (bind _sphere (`self.Sphere`))
  (`/Engine/EditorBlueprintResources/ActorMacros.Switch Has Authority`
    (:`Authority`
      (`self.Explode`)
      (`PrimitiveComponent.SetCollisionResponseToAllChannels` _sphere "ECR_Ignore")
      (`SceneComponent.SetVisibility` _sphere false false)
      (`GameplayStatics.ApplyDamage` Other (`self.Damage`)))))

(event `self.ReceiveTick`
  (params (DeltaSeconds :type "Float (single-precision)"))
  (`/Engine/EditorBlueprintResources/StandardMacros.IsValid` (`self.Trail`)
    (:`Is Valid`
      (`SceneComponent.K2_SetWorldRotation` (`self.Trail`) (`KismetMathLibrary.Conv_VectorToRotator` (`self.GetVelocity`)) false false))
    (:`Is Not Valid`
      (`/Engine/EditorBlueprintResources/ActorMacros.Switch Has Authority`
        (:`Authority`
          (`self.K2_DestroyActor`)
          (`KismetSystemLibrary.PrintString` "Destroydd"))))))

(event `Explode`
  (`GameplayStatics.SpawnEmitterAtLocation` "/Game/Particles/pew.pew" (`self.K2_GetActorLocation`))
  (`ActorComponent.Deactivate` (`self.Trail`)))

(fn `UserConstructionScript`)