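; VectorArrayFunctions is a set of array helper functions that appears unfinished.
; TransferIndices loops from Start to a bound derived from From's length and Step, setting To at stepped indices and printing a debug string each pass.
; The strided read from From is left unconnected, so the set receives no source value before the array is returned.
; LoadNormals is an empty stub.
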(fn `LoadNormals`)

(fn `TransferIndices`
  (params (From :type "Array of Vector Structure") (To :type "Array of Vector Structure (by ref)") (Start :type Integer) (Step :type Integer))
  (returns (NewParam :type "Array of Vector Structure"))
  (locals (a :type "Array of Vector Structure"))
  (set `local.a` To)
  (for _index (range Start (+ (/ (- (`KismetArrayLibrary.Array_LastIndex` From) Start) Step) 1))
    (`KismetArrayLibrary.Array_Set` (`local.a`) (* _index Step))
    (`KismetSystemLibrary.PrintString` null "st"))
  (return (`local.a`)))